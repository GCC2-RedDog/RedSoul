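; BP_Incantation is a player ability that casts a fireball at a mana cost.
; Using checks that the player's CurMana exceeds AbilityUsage, then plays the casting montage, triggers Spawn and calls the parent Using.
; Spawn waits briefly, deducts the mana and spawns BP_FireBall at the player's left-hand socket.
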(event `Spawn`
  (`KismetSystemLibrary.Delay` 0.5)
  (bind _asbp_player (cast `/Game/JS/Blueprints/BP/BP_Player` (`GameplayStatics.GetPlayerPawn` 0)))
  (set `/Game/JS/Blueprints/BP/BP_Player.CurMana` (- (`/Game/JS/Blueprints/BP/BP_Player.CurMana` _asbp_player) (`self.AbilityUsage`)) _asbp_player)
  (`|SpawnActorFromClass` "/Game/JS/Blueprints/BP/BP_FireBall.BP_FireBall_C" (`SceneComponent.GetSocketTransform` (`Character.Mesh` _asbp_player) "hand_lSocket" "RTS_World") "Undefined" "MultiplyWithRoot" null null))

(fn `UserConstructionScript`
  (`parent.UserConstructionScript`))

(fn `Using`
  (bind _asbp_player (cast `/Game/JS/Blueprints/BP/BP_Player` (`GameplayStatics.GetPlayerCharacter` 0)))
  (if (< (`self.AbilityUsage`) (`/Game/JS/Blueprints/BP/BP_Player.CurMana` _asbp_player))
    (`Character.PlayAnimMontage` _asbp_player "/Game/JS/Montage/M_Casting1.M_Casting1" 1.0 "None")
    (`self.Spawn`)
    (`parent.Using`)))
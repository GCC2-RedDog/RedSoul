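; BP_FireBall is a fireball projectile effect that damages the boss on contact.
; On BeginPlay it copies the player pawn's rotation so it faces the player's heading.
; Overlapping a BP_Boss calls its Hit with a non-parryable AttackInfo carrying the Damage value, then destroys the fireball.
; Its own Hit function is an empty stub, and no movement logic appears in the graphs.
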(event `self.ReceiveBeginPlay`
  (`self.K2_SetActorRotation` (`self.K2_GetActorRotation` (`GameplayStatics.GetPlayerPawn` 0))))

(event `self.ReceiveActorBeginOverlap`
  (params (OtherActor :type "Actor Object Reference"))
  (bind _asbp_boss (cast `/Game/SK/Blueprints/BP_Boss` OtherActor))
  (`Hitable.Hit` _asbp_boss (make `AttackInfo` (`self.Damage`)))
  (`self.K2_DestroyActor`))

(fn `Hit`
  (params (AttackInfo :type "AttackInfo Structure"))
  (returns (ReturnValue :type "EAttackResult Enum"))
  (return "AR_None"))

(fn `UserConstructionScript`)
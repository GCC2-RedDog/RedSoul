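; BP_MagicArrow is a projectile that flies at the boss and damages it on overlap.
; On BeginPlay it finds BP_Boss, locks a direction toward it and turns to face it, so it does not home afterward.
; Tick moves it along that line at Speed without sweeping.
; Overlapping the boss sends an unparryable attack through Hit and destroys the arrow, which otherwise expires after a short delay.
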(event `self.ReceiveBeginPlay`
  (bind _returnvalue (`self.K2_GetActorLocation`))
  (bind _returnvalue_2 (`GameplayStatics.GetActorOfClass` "/Game/SK/Blueprints/BP_Boss.BP_Boss_C"))
  (bind _returnvalue_3 (`self.K2_GetActorLocation` _returnvalue_2))
  (set `self.Direction` (`KismetMathLibrary.Normal` (- _returnvalue_3 _returnvalue)))
  (`self.K2_SetActorRotation` (`KismetMathLibrary.FindLookAtRotation` _returnvalue _returnvalue_3))
  (`KismetSystemLibrary.Delay` 4.0)
  (`self.K2_DestroyActor`))

(event `self.ReceiveActorBeginOverlap`
  (params (OtherActor :type "Actor Object Reference"))
  (bind _asbp_boss (cast `/Game/SK/Blueprints/BP_Boss` OtherActor))
  (`Hitable.Hit` _asbp_boss (make `AttackInfo` (`self.Damage`)))
  (`self.K2_DestroyActor`))

(event `self.ReceiveTick`
  (params (DeltaSeconds :type "Float (single-precision)"))
  (`self.K2_SetActorLocation` (+ (`self.K2_GetActorLocation`) (* DeltaSeconds (`self.Speed`) (`self.Direction`)))))

(fn `Hit`
  (params (AttackInfo :type "AttackInfo Structure"))
  (returns (ReturnValue :type "EAttackResult Enum"))
  (return "AR_None"))

(fn `UserConstructionScript`)
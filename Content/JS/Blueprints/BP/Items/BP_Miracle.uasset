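; BP_Miracle is a usable healing item that spends the player's mana to restore HP.
; Using checks that BP_Player has more mana than AbilityUsage, then plays a casting montage, triggers Spawn and calls the parent Using.
; After a short delay, Spawn deducts the mana, adds HealValue to HP without clamping, and spawns BP_Heal at the player's right-hand socket.
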(event `Spawn`
  (`KismetSystemLibrary.Delay` 0.7)
  (bind _asbp_player (cast `/Game/JS/Blueprints/BP/BP_Player` (`GameplayStatics.GetPlayerPawn` 0)))
  (set `/Game/JS/Blueprints/BP/BP_Player.CurMana` (- (`/Game/JS/Blueprints/BP/BP_Player.CurMana` _asbp_player) (`self.AbilityUsage`)) _asbp_player)
  (set `/Game/JS/Blueprints/BP/BP_Player.CurPlayerHp` (+ (`/Game/JS/Blueprints/BP/BP_Player.CurPlayerHp` _asbp_player) (`self.HealValue`)) _asbp_player)
  (`|SpawnActorFromClass` "/Game/JS/Blueprints/BP/Effects/BP_Heal.BP_Heal_C" (`SceneComponent.GetSocketTransform` (`Character.Mesh` _asbp_player) "hand_rSocket" "RTS_World") "Undefined" "MultiplyWithRoot" null null))

(fn `UserConstructionScript`
  (`parent.UserConstructionScript`))

(fn `Using`
  (bind _asbp_player (cast `/Game/JS/Blueprints/BP/BP_Player` (`GameplayStatics.GetPlayerCharacter` 0)))
  (if (< (`self.AbilityUsage`) (`/Game/JS/Blueprints/BP/BP_Player.CurMana` _asbp_player))
    (`Character.PlayAnimMontage` _asbp_player "/Game/JS/Montage/M_Casting2.M_Casting2" 1.0 "None")
    (`self.Spawn`)
    (`parent.Using`)))
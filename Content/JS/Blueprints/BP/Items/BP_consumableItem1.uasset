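; Consumable item that restores the player's mana by its Value when used.
; The Using override fires a custom event, then calls the parent Using without waiting for that event's one-second delay.
; After the delay, it adds Value to BP_Player's CurMana with no clamp here and spawns a BP_ItemUse actor at the mesh's rootSocket.
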(event `CustomEvent`
  (`KismetSystemLibrary.Delay` 1.0)
  (bind _asbp_player (cast `/Game/JS/Blueprints/BP/BP_Player` (`GameplayStatics.GetPlayerPawn` 0)))
  (set `/Game/JS/Blueprints/BP/BP_Player.CurMana` (+ (`/Game/JS/Blueprints/BP/BP_Player.CurMana` _asbp_player) (`self.Value`)) _asbp_player)
  (`|SpawnActorFromClass` "/Game/JS/Blueprints/BP/Effects/BP_ItemUse.BP_ItemUse_C" (`SceneComponent.GetSocketTransform` (`Character.Mesh` _asbp_player) "rootSocket" "RTS_World") "Undefined" "MultiplyWithRoot" null null))

(fn `UserConstructionScript`
  (`parent.UserConstructionScript`))

(fn `Using`
  (`self.CustomEvent`)
  (`parent.Using`))
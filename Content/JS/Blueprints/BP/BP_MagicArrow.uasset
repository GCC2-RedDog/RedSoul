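; BP_MagicArrow is a projectile that flies at the boss and damages it on contact.
; On BeginPlay it finds the BP_Boss in the level and stores a fixed normalized direction toward it, without homing afterward.
; Tick moves it along that direction at Speed without sweeping.
; On overlapping the boss, it calls Hit with non-stunning attack info carrying its Damage, then destroys itself.
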(event `self.ReceiveBeginPlay`
  (bind _returnvalue (`GameplayStatics.GetActorOfClass` "/Game/SK/Blueprints/BP_Boss.BP_Boss_C"))
  (set `self.Direction` (`KismetMathLibrary.Normal` (- (`self.K2_GetActorLocation` _returnvalue) (`self.K2_GetActorLocation`)))))

(event `self.ReceiveActorBeginOverlap`
  (params (OtherActor :type "Actor Object Reference"))
  (bind _asbp_boss (cast `/Game/SK/Blueprints/BP_Boss` OtherActor))
  (`Hitable.Hit` _asbp_boss (make `AttackInfo` (`self.Damage`)))
  (`self.K2_DestroyActor`))

(event `self.ReceiveTick`
  (params (DeltaSeconds :type "Float (single-precision)"))
  (`self.K2_SetActorLocation` (+ (`self.K2_GetActorLocation`) (* DeltaSeconds (`self.Speed`) (`self.Direction`)))))

(fn `UserConstructionScript`)